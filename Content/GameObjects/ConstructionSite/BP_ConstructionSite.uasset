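; BP_ConstructionSite is a construction site actor that visually shows build progress by moving its frame and building components.
; On BeginPlay both components snap to their default offsets.
; OnAdvanced receives a progress amount and state, then linearly interpolates the frame toward the origin during Framing, or the building toward a fixed raised position during Building, both in relative space.
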(event EventOnAdvanced
  (params (InNewAmount :type Float%20%28single-precision%29) (InNewState :type EConstructionState%20Enum :default "Framing"))
  (switch Utilities|FlowControl|Switch|SwitchonEConstructionState InNewState
    (:Framing
      (Transformation|SetRelativeLocation (Variables|Default|GetFrameRoot) (Math|Vector|Lerp(Vector) (Variables|Default|GetFrameDefaultOffset) "0, 0, 0" InNewAmount) false false))
    (:Building
      (Transformation|SetRelativeLocation (Variables|Default|GetBuilding) (Math|Vector|Lerp(Vector) (Variables|Default|GetBuildingDefaultOffset) "0, 0,164.000000" InNewAmount) false false))))

(event EventBeginPlay
  (Transformation|SetRelativeLocation (Variables|Default|GetFrameRoot) (Variables|Default|GetFrameDefaultOffset) false false)
  (Transformation|SetRelativeLocation (Variables|Default|GetBuilding) (Variables|Default|GetBuildingDefaultOffset) false false))

(fn ConstructionScript)