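; BP_GridRenderer is a stress-test actor that draws a square grid of cube cells around its location, randomly marked valid or invalid.
; The construction script clears two instanced mesh components, assigns each its material and a unit cube, and enables custom depth on both.
; A nested loop over the grid dimensions then adds each cell to one component at random, positioned and scaled by the grid spacing.
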(event EventBeginPlay)

(event Collision|EventActorBeginOverlap
  (params (OtherActor :type Actor%20Object%20Reference)))

(event EventTick
  (params (DeltaSeconds :type Float%20%28single-precision%29)))

(fn ConstructionScript
  (bind _validcells (Variables|Default|GetValidCells))
  (bind _griddimensions (Variables|Default|GetGridDimensions))
  (bind _gridspacing (Variables|Default|GetGridSpacing))
  (bind _returnvalue (Math|Conversions|ToVector(Float) _gridspacing))
  (bind _returnvalue_2 (* _griddimensions -1.0))
  (bind _returnvalue_3 (Math|Float|Truncate _returnvalue_2))
  (Rendering|SetRenderCustomDepth _validcells true)
  (Components|InstancedStaticMesh|ClearInstances _validcells)
  (Rendering|Material|SetMaterial (Variables|Default|GetInvalidCells) 0 (Variables|Default|GetInvalidMaterial))
  (Rendering|Material|SetMaterial (Variables|Default|GetValidCells) 0 (Variables|Default|GetValidMaterial))
  (Components|StaticMesh|SetStaticMesh (Variables|Default|GetValidCells) "/Game/StaticMeshes/Primitives/SM_Cube_1x1.SM_Cube_1x1")
  (Components|StaticMesh|SetStaticMesh (Variables|Default|GetInvalidCells) "/Game/StaticMeshes/Primitives/SM_Cube_1x1.SM_Cube_1x1")
  ;[1 1 1] X
  (for _index (range _returnvalue_3 _griddimensions)
    ;[1 1 1] Y
    (for _index_2 (range _returnvalue_3 _griddimensions)
      (if (Math|Random|RandomBool)
        (Class|InstancedStaticMeshComponent|AddInstanceWorldSpace (Variables|Default|GetValidCells) (Math|Transform|MakeTransform (+ (Transformation|GetActorLocation) (Math|Vector|MakeVector (* (Variables|Default|GetGridSpacing) (Math|Conversions|ToFloat(Integer) _index)) (* (Variables|Default|GetGridSpacing) (Math|Conversions|ToFloat(Integer) _index_2)) 0.0)) "0, 0, 0" _returnvalue))
        (else
          (Class|InstancedStaticMeshComponent|AddInstanceWorldSpace (Variables|Default|GetInvalidCells) (Math|Transform|MakeTransform (+ (Transformation|GetActorLocation) (Math|Vector|MakeVector (* (Variables|Default|GetGridSpacing) (Math|Conversions|ToFloat(Integer) _index)) (* (Variables|Default|GetGridSpacing) (Math|Conversions|ToFloat(Integer) _index_2)) 0.0)) "0, 0, 0" _returnvalue)))))))